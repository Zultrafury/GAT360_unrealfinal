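; Player combat component handling target lock-on, sword combos and directional dodging, with stamina costs through the character's stats component.
; Lock-on sphere-traces from the camera, attaches a marker actor and turns control rotation toward the target each tick.
; Attack input during a montage queues the next hit at a notify, while dodge picks its montage by direction key when strafing.
; A looping timer runs sword sphere traces, applying damage behind a short cooldown.
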(event `self.ReceiveBeginPlay`
  ;[0.1042 0.1042 0.1042 0.5] Get Player Class
  (bind _asbp_nycks_third_person_character (cast `/Game/NycksWork/BP_NycksThirdPersonCharacter` (`self.GetOwner`)))
  (set `self.Playerr BP` _asbp_nycks_third_person_character))

(event `EnhancedInput|/Game/Input/Actions/IA_LockOn`
  (params (ActionValue :type Boolean) (ElapsedSeconds :type "Float (double-precision)") (TriggeredSeconds :type "Float (double-precision)") (InputAction :type "InputAction Object Reference" :default "/Game/Input/Actions/IA_LockOn.IA_LockOn"))
  (bind _returnvalue (`Actor.GetTransform` (`self.Target Lock Actor`)))
  (bind _transformcomponent (`PlayerCameraManager.TransformComponent` (`GameplayStatics.GetPlayerCameraManager` 0)))
  (bind _charactermovement (`Character.CharacterMovement` (`self.Playerr BP`)))
  (bind _charactermovement_2 (`Character.CharacterMovement` (`self.Playerr BP`)))
  (bind (_returnvalue_x _returnvalue_y _returnvalue_z) (`KismetMathLibrary.BreakVector` (`SceneComponent.K2_GetComponentLocation` _transformcomponent)))
  (bind _returnvalue_2 (`KismetMathLibrary.MakeVector` _returnvalue_x _returnvalue_y (+ _returnvalue_z 20.0)))
  ;[0.15 0.06829 0.1447 0.5] Vaild Target hit
  (:`Started`
    (`self.Target Lock Actor`
      (:`then`
        (set `self.Target Lock Actor` null)
        (set `CharacterMovementComponent.bOrientRotationToMovement` true _charactermovement)
        (set `CharacterMovementComponent.bUseControllerDesiredRotation` false _charactermovement)
        (`Actor.K2_DestroyActor` (`self.Target Lock Widget`)))
      (:`else`
        (bind (_outhit _returnvalue_3) (`KismetSystemLibrary.SphereTraceSingleForObjects` :`Start` _returnvalue_2 :`End` (+ _returnvalue_2 (* (`KismetMathLibrary.GetForwardVector` (`SceneComponent.K2_GetComponentRotation` _transformcomponent)) 1000.0)) :`Radius` 150.0 :`ObjectTypes` (`|MakeArray` "ObjectTypeQuery3" :!type "EObjectTypeQuery Enum") :`DrawDebugType` "ForDuration" :`DrawTime` 2.0))
        (if _returnvalue_3
          (set `self.Target Lock Actor` (`.HitActor` (`GameplayStatics.BreakHitResult` _outhit)))
          (set `CharacterMovementComponent.bOrientRotationToMovement` false _charactermovement_2)
          (set `CharacterMovementComponent.bUseControllerDesiredRotation` true _charactermovement_2)
          (bind _returnvalue_4 (`|SpawnActorFromClass` "/Game/NycksWork/Blueprints/BP_TargetLockWidget.BP_TargetLockWidget_C" (`KismetMathLibrary.MakeTransform` (`KismetMathLibrary.MakeVector` (.x (.location _returnvalue)) (.y (.location _returnvalue)) (+ (.z (.location _returnvalue)) 20.0)) (.rotation _returnvalue)) "AlwaysSpawn" "MultiplyWithRoot" null null))
          (bind _output_get (set `self.Target Lock Widget` _returnvalue_4))
          (`Actor.K2_AttachToActor` _output_get (`self.Target Lock Actor`) "None" "SnapToTarget" "SnapToTarget" "SnapToTarget" true))))))

(event `self.ReceiveTick`
  (params (DeltaSeconds :type "Float (single-precision)"))
  (bind (_returnvalue_roll _returnvalue_pitch _returnvalue_yaw) (`KismetMathLibrary.BreakRotator` (`KismetMathLibrary.FindLookAtRotation` (`Actor.K2_GetActorLocation` (`self.Playerr BP`)) (`Actor.K2_GetActorLocation` (`self.Target Lock Actor`)))))
  ;[0.15 0.06829 0.1447 0.5] Target Lock Update
  (`self.Target Lock Actor`
    (:`then`
      (`Controller.SetControlRotation` (`Pawn.GetController` (`self.Playerr BP`)) (`KismetMathLibrary.MakeRotator` _returnvalue_roll (+ _returnvalue_pitch -20.0) _returnvalue_yaw)))
    (:`else`)))

(event `EnhancedInput|/Game/Input/Actions/IA_Attack`
  (params (ActionValue :type Boolean) (ElapsedSeconds :type "Float (double-precision)") (TriggeredSeconds :type "Float (double-precision)") (InputAction :type "InputAction Object Reference" :default "/Game/Input/Actions/IA_Attack.IA_Attack"))
  (bind _bpc_stats (`/Game/NycksWork/BP_NycksThirdPersonCharacter.BPC_Stats` (`self.Playerr BP`)))
  ;[0.1046 0.0185 0.02843 0.502] Sword Combo Animation
  (:`Started`
    (if (and (not (`self.IsAttacking`)) (>= (`/Game/NycksWork/Blueprints/BPC_Stats.stamina` (`/Game/NycksWork/BP_NycksThirdPersonCharacter.BPC_Stats` (`self.Playerr BP`))) 10.0) (`/Game/NycksWork/BP_NycksThirdPersonCharacter.weaponEquipped` (`self.Playerr BP`)))
      (set `self.IsAttacking` true)
      (`|PlayMontage` (`Character.Mesh` (`self.Playerr BP`)) "/Game/NycksWork/Animations/Attacks/SwordAttackCombo_Montage.SwordAttackCombo_Montage"
        (:`then`
          (set `/Game/NycksWork/Blueprints/BPC_Stats.RegainStamina` false _bpc_stats)
          (`/Game/NycksWork/Blueprints/BPC_Stats.Increase Value` _bpc_stats "NewEnumerator1" -10.0 :!label _label))
        (:`OnCompleted`
          (set `self.IsAttacking` false :!label _label_2)
          (set `self.Combo?` false)
          (set `/Game/NycksWork/Blueprints/BPC_Stats.RegainStamina` true (`/Game/NycksWork/BP_NycksThirdPersonCharacter.BPC_Stats` (`self.Playerr BP`))))
        (:`OnInterrupted`
          (goto _label_2))
        (:`OnNotifyBegin`
          (if (and (`self.IsAttacking`) (`self.Combo?`))
            (set `self.Combo?` false)
            (goto _label)
            (else
              (`AnimInstance.Montage_Stop` (`SkeletalMeshComponent.GetAnimInstance` (`Character.Mesh` (`self.Playerr BP`))) 0.2 "/Game/NycksWork/Animations/Attacks/SwordAttackCombo_Montage.SwordAttackCombo_Montage")))))
      (else
        (set `self.Combo?` true)))))

(event `EnhancedInput|/Game/Input/Actions/IA_Dodge`
  (params (ActionValue :type Boolean) (ElapsedSeconds :type "Float (double-precision)") (TriggeredSeconds :type "Float (double-precision)") (InputAction :type "InputAction Object Reference" :default "/Game/Input/Actions/IA_Dodge.IA_Dodge"))
  (bind _bpc_stats (`/Game/NycksWork/BP_NycksThirdPersonCharacter.BPC_Stats` (`self.Playerr BP`)))
  ;[0.09454 0.1042 0.02549 0.5] Dodege Movement
  (:`Started`
    (if (and (not (`self.IsRolling`)) (>= (`/Game/NycksWork/Blueprints/BPC_Stats.stamina` (`/Game/NycksWork/BP_NycksThirdPersonCharacter.BPC_Stats` (`self.Playerr BP`))) 25.0))
      (set `self.IsRolling` true)
      (`|ExecutionSequence`
        (:`then_0`
          (if (`CharacterMovementComponent.bUseControllerDesiredRotation` (`Character.CharacterMovement` (`self.Playerr BP`)))
            (switch `string` (`KismetTextLibrary.Conv_TextToString` (`KismetInputLibrary.Key_GetDisplayName` (`/Game/NycksWork/BP_NycksThirdPersonCharacter.Direction Key` (`self.Playerr BP`))))
              (:`W`
                (set `self.MovementDirection` "NewEnumerator0"))
              (:`A`
                (set `self.MovementDirection` "NewEnumerator1"))
              (:`S`
                (set `self.MovementDirection` "NewEnumerator2"))
              (:`D`
                (set `self.MovementDirection` "NewEnumerator3")))
            (else
              (set `self.MovementDirection` "NewEnumerator0"))))
        (:`then_1`
          (`|PlayMontage` (`Character.Mesh` (`self.Playerr BP`)) (select `/Game/NycksWork/Blueprints/E_MovementDirection` (`self.MovementDirection`) :`NewEnumerator0` "/Game/NycksWork/Animations/Dodge/Dodge_F_Montage.Dodge_F_Montage" :`NewEnumerator1` "/Game/NycksWork/Animations/Dodge/Dodge_L_Montage.Dodge_L_Montage" :`NewEnumerator2` "/Game/NycksWork/Animations/Dodge/Dodge_B_Montage.Dodge_B_Montage" :`NewEnumerator3` "/Game/NycksWork/Animations/Dodge/Dodge_R_Montage.Dodge_R_Montage" :!type "AnimMontage Object Reference")
            (:`then`
              (set `/Game/NycksWork/Blueprints/BPC_Stats.RegainStamina` false _bpc_stats)
              (`/Game/NycksWork/Blueprints/BPC_Stats.Increase Value` _bpc_stats "NewEnumerator1" -25.0))
            (:`OnCompleted`
              (set `self.IsRolling` false :!label _label_3)
              (set `/Game/NycksWork/Blueprints/BPC_Stats.RegainStamina` true (`/Game/NycksWork/BP_NycksThirdPersonCharacter.BPC_Stats` (`self.Playerr BP`))))
            (:`OnInterrupted`
              (goto _label_3))))))))

(event `Begin Damage Trace`
  ;[0.1046 0.0185 0.02843 0.502] Sword Traces
  (bind _returnvalue (`KismetSystemLibrary.K2_SetTimerDelegate` (delegate `Damage Trace`) 0.1 true)))

(event `End Damage Trace`
  ;[0.1046 0.0185 0.02843 0.502] Sword Traces
  (if (`KismetSystemLibrary.K2_IsValidTimerHandle` (stale `Begin Damage Trace` _returnvalue))
    (`KismetSystemLibrary.K2_ClearAndInvalidateTimerHandle` (stale `Begin Damage Trace` _returnvalue))))

(event `Damage Trace`
  (bind (_playerr_bp _playerr_bp_2) (`self.Playerr BP`))
  ;[0.1046 0.0185 0.02843 0.502] Sword Traces
  (bind (_outhit _returnvalue) (`KismetSystemLibrary.SphereTraceSingleForObjects` :`Start` (`SceneComponent.K2_GetComponentLocation` (`/Game/ThirdPerson/Blueprints/BP_ThirdPersonCharacter.Start Sword Trace Pos` _playerr_bp_2)) :`End` (`SceneComponent.K2_GetComponentLocation` (`/Game/ThirdPerson/Blueprints/BP_ThirdPersonCharacter.End Sword Trace Pos` _playerr_bp_2)) :`Radius` 40.0 :`ObjectTypes` (`|MakeArray` "ObjectTypeQuery3" :!type "EObjectTypeQuery Enum") :`DrawDebugType` "ForOneFrame"))
  (if _returnvalue
    (`/Engine/EditorBlueprintResources/StandardMacros.DoOnce` false :!label _label_4
      (:`Completed`
        (bind (_bblockinghit _binitialoverlap _time _distance _location _impactpoint _normal _impactnormal _physmat _hitactor) (`GameplayStatics.BreakHitResult` _outhit))
        (`GameplayStatics.ApplyDamage` _hitactor (`self.SwordDamage`))
        (`GameplayStatics.PlaySoundAtLocation` "/Game/NycksWork/Audio/MS_Damage.MS_Damage" _location (struct) 1.0 1.0 0.0 null null null null)
        (`GameplayStatics.SpawnEmitterAtLocation` null _location (struct) (1.0 1.0 1.0) true "AutoRelease")
        (`KismetSystemLibrary.Delay` 0.3)
        (goto _label_4 :!via `Reset`)))))