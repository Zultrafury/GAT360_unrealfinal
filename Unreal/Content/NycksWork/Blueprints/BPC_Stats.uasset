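; BPC_Stats is a stats component that tracks Health and Stamina for its owning actor.
; IncreaseValue applies a change to either stat, clamps it between zero and its maximum, and updates that stat's externally assigned progress bar.
; When health reaches zero, it sends DieMessage to the owner.
; A looping timer started on BeginPlay steadily restores stamina while the RegainStamina flag is set.
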(event `self.ReceiveBeginPlay`
  (`KismetSystemLibrary.K2_SetTimerDelegate` (delegate `Regain Stamina`) 0.1 true))

(event `Regain Stamina`
  (if (`self.RegainStamina`)
    (`self.Increase Value` "NewEnumerator1" 1.0)))

(event `Die`
  (message `/Game/NycksWork/Blueprints/BPI_Damage.Die` (`self.GetOwner`)))

(event `Set Health Progress Bar`
  (params (`Health Progress Bar ` :type "ProgressBar Object Reference"))
  (set `self.Health Progress Bar` `Health Progress Bar `))

(event `Set Stamina Progress Bar`
  (params (`Stamina Progress Bar` :type "ProgressBar Object Reference"))
  (set `self.Stamina Progress Bar` `Stamina Progress Bar`))

(fn `Increase Value`
  (params (Stat :type "/Game/NycksWork/Blueprints/E_Stats Enum" :default "NewEnumerator0") (Value :type "Float (double-precision)"))
  ;[0.8281 0 0 0.3739] Health Stats
  (switch `/Game/NycksWork/Blueprints/E_Stats` Stat
    (:`NewEnumerator0`
      (set `self.health` (`KismetMathLibrary.FClamp` (+ (`self.health`) Value) 0.0 (`self.MaxHealth`)))
      (`|ExecutionSequence`
        (:`then_0`
          (if (<= (`self.health`) 0.0)
            (`self.Die`)))
        (:`then_1`
          (bind _health_progress_bar (`self.Health Progress Bar`)
            (:`then`
              (`ProgressBar.SetPercent` _health_progress_bar (/ (`self.health`) (`self.MaxHealth`))))
            (:`else`)))))
    (:`NewEnumerator1`
      ;[0 0.3385 0.00048 0.4725] Stamina
      (set `self.stamina` (`KismetMathLibrary.FClamp` (+ (`self.stamina`) Value) 0.0 (`self.MaxStamina`)))
      (bind _stamina_progress_bar (`self.Stamina Progress Bar`)
        (:`then`
          (`ProgressBar.SetPercent` _stamina_progress_bar (/ (`self.stamina`) (`self.MaxStamina`))))
        (:`else`)))))