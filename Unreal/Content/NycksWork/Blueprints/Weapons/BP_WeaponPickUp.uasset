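; BP_WeaponPickUp is a weapon pickup that hands its weapon data to whatever actor walks into it.
; The construction script sets the static mesh from WeaponData, so each instance shows the weapon it grants.
; On trigger overlap, an actor implementing BPI_Interact receives WeaponData through PickupWeaponMessage, then the pickup plays a sword sound and destroys itself.
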(event `self.Pickup Trigger.OnComponentBeginOverlap`
  (params (OverlappedComponent :type "PrimitiveComponent Object Reference") (OtherActor :type "Actor Object Reference") (OtherComp :type "PrimitiveComponent Object Reference") (OtherBodyIndex :type Integer) (bFromSweep :type Boolean) (SweepResult :type "HitResult Structure (by ref)"))
  (if (`KismetSystemLibrary.DoesImplementInterface` OtherActor "/Game/NycksWork/Blueprints/Weapons/BPI_Interact.BPI_Interact_C")
    (message `/Game/NycksWork/Blueprints/Weapons/BPI_Interact.Pickup Weapon` OtherActor (`self.weaponData`))
    (`GameplayStatics.PlaySoundAtLocation` "/Game/NycksWork/Audio/sword-sound-260274.sword-sound-260274" (`self.K2_GetActorLocation`) (struct) 0.8 1.0 0.0 null null null null)
    (`self.K2_DestroyActor`)))

(fn `UserConstructionScript`
  (`StaticMeshComponent.SetStaticMesh` (`self.StaticMesh`) (`/Game/NycksWork/Blueprints/Weapons/BP_DA_Weapon.StaticMesh` (`self.weaponData`))))