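; Boss enemy Blueprint with a sword attack and a trigger area for showing its health bar.
; BeginPlay runs the parent logic, then reads world locations for the sword trace start and end points.
; When the third-person character enters the trigger, it creates a widget and calls for the boss health bar to be displayed and bound to the stats component.
; SwordAttack plays the attack montage with a sound at the boss's location.
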(event `self.ReceiveBeginPlay`
  (`parent.ReceiveBeginPlay`)
  (set `self.BossStartSwordTracePos` (`SceneComponent.K2_GetComponentLocation` (`self.Boss Start Sword Trace Pos`)))
  (set `self.BossEndSwordTracePos` (`SceneComponent.K2_GetComponentLocation` (`self.Boss End Sword Trace Pos`))))

(event `self.TriggerArea.OnComponentBeginOverlap`
  (params (OverlappedComponent :type "PrimitiveComponent Object Reference") (OtherActor :type "Actor Object Reference") (OtherComp :type "PrimitiveComponent Object Reference") (OtherBodyIndex :type Integer) (bFromSweep :type Boolean) (SweepResult :type "HitResult Structure (by ref)"))
  (cast `/Game/ThirdPerson/Blueprints/BP_ThirdPersonCharacter` OtherActor)
  (bind _returnvalue (`|CreateWidget` null))
  (bind (_output_get _output_get_2) (set `self.BossHealthWidget` null _returnvalue))
  (`UserWidget.AddToViewport` _output_get_2 0)
  (`self.Set Health Progress Bar` (`self.BPC_Stats`) (`/Game/NycksWork/AI/BP_Enemy_Boss.HealthBar` (`.BossHealthWidget` (`self.BossHealthWidget`)))))

(fn `SwordAttack`
  (returns (Duration :type "Float (double-precision)"))
  (bind _returnvalue (`self.PlayAnimMontage` (`self.SwordAttackMontage `)))
  (`GameplayStatics.PlaySoundAtLocation` null (`self.K2_GetActorLocation`) (struct) 1.0 1.0 0.0 null null null null)
  (return _returnvalue))

(fn `UserConstructionScript`
  (`parent.UserConstructionScript`))