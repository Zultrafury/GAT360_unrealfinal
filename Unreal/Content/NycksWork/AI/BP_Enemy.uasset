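; BP_Enemy is a melee enemy, with a boss variant, that has sword and big attack montages, a health bar and ragdoll death.
; BPCStats takes incoming damage and receives the widget's health bar.
; A looping timer runs sword sphere traces between selectable start and end points, throttled by a resetting DoOnce.
; Big attack impacts use a point sphere trace with sound, particles and camera shake; both trigger overlap events show the widget.
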(event `self.ReceiveBeginPlay`
  ;[0.1042 0.1042 0.1042 0.5] Enemy Health
  (bind _aswb_enemy_health (cast `` (`WidgetComponent.GetWidget` (`self.Widget`))))
  (`self.Set Health Progress Bar` (`self.BPC_Stats`) (`/Game/NycksWork/AI/BP_Enemy.HealthBar` _aswb_enemy_health))
  (`SkinnedMeshComponent.HideBoneByName` (`self.Enemy`) "weapon_r" "PBO_None"))

(event `self.ReceiveAnyDamage`
  (params (Damage :type "Float (single-precision)") (DamageType :type "DamageType Object Reference") (InstigatedBy :type "Controller Object Reference") (DamageCauser :type "Actor Object Reference"))
  ;[0.1042 0.1042 0.1042 0.5] Enemy Health
  (`self.Increase Value` (`self.BPC_Stats`) 0 (* Damage -1.0)))

(event `self.End Sword Trace `
  ;[0.1042 0.1042 0.1042 0.5] Sword Traces
  (if (`KismetSystemLibrary.K2_IsValidTimerHandle` (stale `self.Begin Sword Trace` _returnvalue))
    (`KismetSystemLibrary.K2_ClearAndInvalidateTimerHandle` (stale `self.Begin Sword Trace` _returnvalue))))

(event `self.Begin Sword Trace`
  ;[0.1042 0.1042 0.1042 0.5] Sword Traces
  (bind _returnvalue (`KismetSystemLibrary.K2_SetTimerDelegate` (delegate `Damage Trace`) 0.1 true)))

(event `Damage Trace`
  ;[0.1042 0.1042 0.1042 0.5] Sword Traces
  (if (not (`self.isDead`))
    (bind (_outhit _returnvalue) (`KismetSystemLibrary.SphereTraceSingleForObjects` :`Start` (`KismetMathLibrary.SelectVector` (`self.BossStartSwordTracePos`) (`SceneComponent.K2_GetComponentLocation` (`self.Start Pos`)) (`self.IsBoss`)) :`End` (`KismetMathLibrary.SelectVector` (`self.BossEndSwordTracePos`) (`SceneComponent.K2_GetComponentLocation` (`self.End Pos`)) (`self.IsBoss`)) :`Radius` (`self.SwordAttackRadius`) :`ObjectTypes` (`|MakeArray` "ObjectTypeQuery3" :!type "EObjectTypeQuery Enum") :`DrawDebugType` "ForOneFrame"))
    (if _returnvalue
      (`/Engine/EditorBlueprintResources/StandardMacros.DoOnce` false :!label _label
        (:`Completed`
          (`GameplayStatics.ApplyDamage` (`.HitActor` (`GameplayStatics.BreakHitResult` _outhit)) (`self.SwordDamage`))
          (`KismetSystemLibrary.Delay` 0.3)
          (goto _label :!via `Reset`))))))

(event `self.Die`
  ;[0.1042 0.1042 0.1042 0.5] Die
  (`CharacterMovementComponent.DisableMovement` (`self.CharacterMovement`))
  (`SkeletalMeshComponent.SetDisableAnimCurves` (`self.Enemy`) true)
  (`PrimitiveComponent.SetSimulatePhysics` (`self.Mesh`) true)
  (set `self.isDead` true))

(event `self.Point Damage Trace`
  (bind _returnvalue (`SceneComponent.K2_GetComponentLocation` (`self.Point Trace Pos`)))
  (bind _returnvalue_2 (`SceneComponent.K2_GetComponentLocation` (`self.Point Trace Pos`)))
  ;[0.1042 0.1042 0.1042 0.5] Big Attack Trace
  (`|ExecutionSequence`
    (:`then_0`
      (bind (_outhit _returnvalue_3) (`KismetSystemLibrary.SphereTraceSingleForObjects` :`Start` _returnvalue_2 :`End` _returnvalue_2 :`Radius` (`self.PointAttackRadius`) :`ObjectTypes` (`|MakeArray` "ObjectTypeQuery3" :!type "EObjectTypeQuery Enum") :`DrawDebugType` "ForDuration"))
      (if _returnvalue_3
        (`GameplayStatics.ApplyDamage` (`.HitActor` (`GameplayStatics.BreakHitResult` _outhit)) 10.0)))
    (:`then_1`
      (`GameplayStatics.PlaySoundAtLocation` null _returnvalue (struct) 1.0 1.0 0.0 null null null null)
      (`GameplayStatics.PlayWorldCameraShake` null _returnvalue 0.0 2000.0)
      (`GameplayStatics.SpawnEmitterAtLocation` null _returnvalue (struct) (1.0 1.0 1.0) true "AutoRelease"))))

(event `self.Trigger.OnComponentBeginOverlap`
  (params (OverlappedComponent :type "PrimitiveComponent Object Reference") (OtherActor :type "Actor Object Reference") (OtherComp :type "PrimitiveComponent Object Reference") (OtherBodyIndex :type Integer) (bFromSweep :type Boolean) (SweepResult :type "HitResult Structure (by ref)"))
  (if (`KismetSystemLibrary.DoesImplementInterface` OtherActor)
    (`SceneComponent.SetVisibility` (`self.Widget`) true false)))

(event `self.Trigger.OnComponentEndOverlap`
  (params (OverlappedComponent :type "PrimitiveComponent Object Reference") (OtherActor :type "Actor Object Reference") (OtherComp :type "PrimitiveComponent Object Reference") (OtherBodyIndex :type Integer))
  (if (`KismetSystemLibrary.DoesImplementInterface` OtherActor)
    (`SceneComponent.SetVisibility` (`self.Widget`) true false)))

(fn `BigAttack`
  (returns (Duration :type "Float (double-precision)"))
  (bind _returnvalue (`self.PlayAnimMontage` (`self.BigAttackMontage`)))
  (`GameplayStatics.PlaySoundAtLocation` null (`self.K2_GetActorLocation`) (struct) 1.0 1.0 0.0 null null null null)
  (return _returnvalue))

(fn `SwordAttack`
  (returns (Duration :type "Float (double-precision)"))
  (bind _returnvalue (`self.PlayAnimMontage` (`self.SwordAttackMontage `)))
  (`GameplayStatics.PlaySoundAtLocation` null (`self.K2_GetActorLocation`) (struct) 1.0 1.0 0.0 null null null null)
  (return _returnvalue))

(fn `UserConstructionScript`)